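; TriArmGameInstance is the game instance that manages the pause menu, level restarts and localisation display data lookup.
; It creates a single UI_PauseMenu widget, injects itself before telling it to pause, then unpauses and removes it on destroy.
; Restarting clears the menu, opens the starting level by name and sets game-only input on the player controller cached at Init.
; A map lookup returns display data for a culture key.
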(event Custom|RestartLevel_Event
  (CallFunction|RestartLevel))

(event EventInit
  (CallFunction|RefreshPlayerController))

(fn GeneratePauseMenu
  (Utilities|IsValid (Variables|Default|GetUIPauseMenuReference)
    (:Is%20Valid
      (return))
    (:Is%20Not%20Valid
      (bind _returnvalue (UserInterface|CreateWidget "/Game/0Project/Jetsources/UI/UI_PauseMenu.UI_PauseMenu_C"))
      ;[1 1 1] Inject Before Pausing
      (bind _output_get (Variables|Default|SetUIPauseMenuReference _returnvalue))
      (UserInterface|Viewport|AddtoViewport _output_get 0)
      (Default|InjectTriArmGameInstance _output_get self)
      (Default|PauseGame _output_get))))

(fn RefreshPlayerController
  (bind _output_get (Variables|Default|SetPlayerController0 (Game|GetPlayerController 0)))
  (return _output_get))

(fn DestroyPauseMenu
  (if (Utilities|IsValid (Variables|Default|GetUIPauseMenuReference))
    (Default|UnpauseGame (Variables|Default|GetUIPauseMenuReference))
    (Widget|RemovefromParent (Variables|Default|GetUIPauseMenuReference))
    (Variables|TriArmGameInstance_C|SetUIPauseMenuReference self 0)
    (else
      (return))))

(fn RestartLevel
  ;[1 1 1] Restart the level
  (CallFunction|DestroyPauseMenu)
  (Game|OpenLevel(byName) (Variables|Default|GetStartingLevelName))
  (Input|SetInputModeGameOnly (Variables|Default|GetPlayerController0)))

(fn GetLocalisationDisplayData
  (params (CultureKey :type String))
  (bind _localisationdisplaydata (Variables|Default|GetLocalisationDisplayData))
  (bind (_value _returnvalue) (Utilities|Map|Find _localisationdisplaydata CultureKey))
  (return _returnvalue _value))